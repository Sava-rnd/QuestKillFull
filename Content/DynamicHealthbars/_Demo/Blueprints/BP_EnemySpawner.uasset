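; Demo enemy spawner actor for the dynamic healthbars showcase that spawns BP_Enemy characters and sends them running to a given location.
; Its SpawnEnemy event creates an enemy at its own transform with a chosen healthbar variation, plus a spawn particle effect.
; It spawns the enemy's default controller, hands over the destination and a back-reference to itself, then triggers the run after a short delay.
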(event `SpawnEnemy`
  (params (HealthbarVariationIndex :type Integer) (RunToLocation :type "Actor Object Reference"))
  ;[1 1 1] Spawn an enemy and get it to run to the specified location
  (bind _returnvalue (`|SpawnActorFromClass` "/Game/DynamicHealthbars/_Demo/_ThirdPersonEnemy/ThirdPersonEnemy/BP_Enemy.BP_Enemy_C" (`KismetMathLibrary.MakeTransform` (`self.K2_GetActorLocation`) (`self.K2_GetActorRotation`)) "Undefined" "OverrideRootScale" self HealthbarVariationIndex null))
  (`GameplayStatics.SpawnEmitterAtLocation` "/Game/DynamicHealthbars/_Demo/FX/EnemySpawn/P_EnemySpawn.P_EnemySpawn" (`self.K2_GetActorLocation`) (struct) (4.0 4.0 4.0))
  (`Pawn.SpawnDefaultController` _returnvalue)
  (set `/Game/DynamicHealthbars/_Demo/_ThirdPersonEnemy/ThirdPersonEnemy/BP_Enemy.RunToLocation` RunToLocation _returnvalue)
  (set `/Game/DynamicHealthbars/_Demo/_ThirdPersonEnemy/ThirdPersonEnemy/BP_Enemy.EnemySpawner` self _returnvalue)
  (`KismetSystemLibrary.Delay` 0.25)
  (`/Game/DynamicHealthbars/_Demo/_ThirdPersonEnemy/ThirdPersonEnemy/BP_Enemy.AttemptRunToLocation` _returnvalue))

(fn `UserConstructionScript`)