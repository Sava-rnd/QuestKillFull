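; BP_Door_Basement_A is an interactive basement door that opens and closes with the E key.
; Overlapping its Trigger enables player input on the actor, and leaving disables it.
; E plays or reverses a timeline that drives the door's yaw, with IsClosed updated from whether that yaw is still above the -120 degree open threshold.
; The construction script applies a configurable material to the door mesh.
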(event `self.Trigger.OnComponentBeginOverlap`
  (params (OverlappedComponent :type "PrimitiveComponent Object Reference") (OtherActor :type "Actor Object Reference") (OtherComp :type "PrimitiveComponent Object Reference") (OtherBodyIndex :type Integer) (bFromSweep :type Boolean) (SweepResult :type "HitResult Structure (by ref)"))
  (`self.EnableInput` (`GameplayStatics.GetPlayerController` 0)))

(event `Key|E`
  (params (Key :type "Key Structure"))
  (:`Pressed`
    (if (`self.IsClosed`)
      (bind (_direction _newtrack_1) (`Timeline|Timeline_0` :!label _label)
        (:`Update`
          (`SceneComponent.K2_SetRelativeRotation` (`self.Door`) (`KismetMathLibrary.MakeRotator` 0.0 0.0 _newtrack_1) false false)
          (if (> _newtrack_1 -120.0)
            (set `self.IsClosed` true)
            (else
              (set `self.IsClosed` false)))))
      (else
        (goto _label :!via `Reverse`)))))

(event `self.Trigger.OnComponentEndOverlap`
  (params (OverlappedComponent :type "PrimitiveComponent Object Reference") (OtherActor :type "Actor Object Reference") (OtherComp :type "PrimitiveComponent Object Reference") (OtherBodyIndex :type Integer))
  (`self.DisableInput` (`GameplayStatics.GetPlayerController` 0)))

(fn `UserConstructionScript`
  (`PrimitiveComponent.SetMaterial` (`self.Door`) 0 (`self.Element 0`)))