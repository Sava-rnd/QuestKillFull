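; AN_Footstep is an animation notify that plays surface-based footstep sounds and reports their noise to AI perception.
; It traces down from the mesh owner against world objects and picks grass or concrete audio from the hit surface, with stone and rock sharing concrete.
; When the owner's ability system has the stealth tag, the owner's sneak value reduces both volume and noise loudness.
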(fn `Received_Notify`
  (params (MeshComp :type "SkeletalMeshComponent Object Reference") (Animation :type "AnimSequenceBase Object Reference") (EventReference :type "AnimNotifyEventReference Structure (by ref)"))
  (returns (ReturnValue :type Boolean))
  (bind _returnvalue (`Actor.K2_GetActorLocation` (`ActorComponent.GetOwner` MeshComp)))
  (bind _returnvalue_2 (`ActorComponent.GetOwner` (`local.MeshComp`)))
  (bind (_outhit _returnvalue_3) (`KismetSystemLibrary.LineTraceSingleForObjects` _returnvalue (- _returnvalue (0.0 0.0 150.0)) (`|MakeArray` "ObjectTypeQuery1" "ObjectTypeQuery2" :!type "EObjectTypeQuery Enum")))
  (if _returnvalue_3
    (bind _result (message `/Game/Postal2/Blueprint/Core/Character/Interfaces/BPI_CharacterHelper.GetSneak` _returnvalue_2))
    (bind (_bblockinghit _binitialoverlap _time _distance _location) (`GameplayStatics.BreakHitResult` _outhit))
    (bind _returnvalue_4 (`KismetMathLibrary.SelectFloat` (- 1.0 _result) 1.0 (`GameplayTagAssetInterface.HasMatchingGameplayTag` (`AbilitySystemBlueprintLibrary.GetAbilitySystemComponent` _returnvalue_2) (struct :`TagName` "Status.Character.InStealth"))))
    (`GameplayStatics.PlaySoundAtLocation` (select `EPhysicalSurface` (`GameplayStatics.GetSurfaceType` _outhit) :`SurfaceType_Default` "/Game/Postal2/Blueprint/Audio/Footsteps/MSS_Footstep_Concrete.MSS_Footstep_Concrete" :`SurfaceType1` "/Game/Postal2/Blueprint/Audio/Footsteps/MSS_Footstep_Grass.MSS_Footstep_Grass" :`SurfaceType2` "/Game/Postal2/Blueprint/Audio/Footsteps/MSS_Footstep_Concrete.MSS_Footstep_Concrete" :`SurfaceType3` "/Game/Postal2/Blueprint/Audio/Footsteps/MSS_Footstep_Concrete.MSS_Footstep_Concrete" :`SurfaceType4` "/Game/Postal2/Blueprint/Audio/Footsteps/MSS_Footstep_Concrete.MSS_Footstep_Concrete" :!type "SoundBase Object Reference") _location (struct) _returnvalue_4 1.0 0.0 "/Game/Postal2/Blueprint/Audio/Footsteps/SA_Footstep.SA_Footstep" null null null)
    (`AISense_Hearing.ReportNoiseEvent` _location _returnvalue_4 (`ActorComponent.GetOwner` (`local.MeshComp`)) 2000.0)
    (return true)
    (else
      (return false))))