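; Player controller for the Postal player character that handles Enhanced Input movement and look, the pause menu and the quest log.
; BeginPlay adds the input mapping context and caches the possessed BP_SkeletonPlayer and its movement component, which receives camera-relative move input directly.
; The pause action toggles game pause, a reused menu widget, input mode and cursor.
; Tab creates a quest log widget when the active-quest query passes.
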(event `Key|Tab`
  (params (Key :type "Key Structure"))
  (bind (_datatable_datatable _datatable_rowname) (break `DataTableRowHandle` (`self.DataTable`)))
  (:`Pressed`
    (if (`/Game/Postal2/Blueprint/Core/GameSystem/QuestSystem/QuestLogComponent.QueryActiveQuest` (`/Game/Postal2/Blueprint/Core/Character/BP_SkeletonPlayer.QuestLogComponent` (`self.BP Skeleton Player`)) _datatable_rowname)
      (bind _returnvalue (`|CreateWidget` "/Game/Postal2/Blueprint/Core/GameSystem/QuestSystem/UI/W_QuestLog.W_QuestLog_C"))
      (bind _output_get (set `self.W_QuestLog` _returnvalue))
      (`UserWidget.AddToViewport` _output_get 0))))

(event `self.ReceiveBeginPlay`
  (`WidgetBlueprintLibrary.SetInputMode_GameOnly` self)
  (set `self.bShowMouseCursor` false)
  (`EnhancedInputSubsystemInterface.AddMappingContext` (subsystem `EnhancedInputLocalPlayerSubsystem`) "/Game/Postal2/Blueprint/Core/EnhancedInput/IMC_PostalInput.IMC_PostalInput" 0 (struct))
  (bind _asbp_skeleton_player (cast `/Game/Postal2/Blueprint/Core/Character/BP_SkeletonPlayer` (`self.K2_GetPawn`)))
  (bind _output_get (set `self.BP Skeleton Player` _asbp_skeleton_player))
  (set `self.CharacterMovementComp` (`Character.CharacterMovement` _output_get)))

(event `EnhancedInput|/Game/Postal2/Blueprint/Core/EnhancedInput/Action/IA_PostalMove`
  (params (ActionValue :type "Vector2D Structure") (ElapsedSeconds :type "Float (double-precision)") (TriggeredSeconds :type "Float (double-precision)") (InputAction :type "InputAction Object Reference" :default "/Game/Postal2/Blueprint/Core/EnhancedInput/Action/IA_PostalMove.IA_PostalMove"))
  (bind (_returnvalue_roll _returnvalue_pitch _returnvalue_yaw) (`KismetMathLibrary.BreakRotator` (`self.GetControlRotation`)))
  (bind (_returnvalue_roll_2 _returnvalue_pitch_2 _returnvalue_yaw_2) (`KismetMathLibrary.BreakRotator` (`self.GetControlRotation`)))
  (:`Triggered`
    (bind _charactermovementcomp (`self.CharacterMovementComp`)
      (:`then`
        (`|ExecutionSequence`
          (:`then_0`
            (`PawnMovementComponent.AddInputVector` _charactermovementcomp (* (`KismetMathLibrary.GetForwardVector` (`KismetMathLibrary.MakeRotator` 0.0 0.0 _returnvalue_yaw)) ActionValue_Y) false))
          (:`then_1`
            (`PawnMovementComponent.AddInputVector` _charactermovementcomp (* (`KismetMathLibrary.GetRightVector` (`KismetMathLibrary.MakeRotator` _returnvalue_roll_2 0.0 _returnvalue_yaw_2)) ActionValue_X) false))))
      (:`else`))))

(event `EnhancedInput|/Game/Postal2/Blueprint/Core/EnhancedInput/Action/IA_PostalLook`
  (params (ActionValue :type "Vector2D Structure") (ElapsedSeconds :type "Float (double-precision)") (TriggeredSeconds :type "Float (double-precision)") (InputAction :type "InputAction Object Reference" :default "/Game/Postal2/Blueprint/Core/EnhancedInput/Action/IA_PostalLook.IA_PostalLook"))
  (:`Triggered`
    (`self.AddYawInput` ActionValue_X)
    (`self.AddPitchInput` ActionValue_Y)))

(event `EnhancedInput|/Game/Postal2/Blueprint/Core/EnhancedInput/Action/IA_PostalPauseMenu`
  (params (ActionValue :type Boolean) (ElapsedSeconds :type "Float (double-precision)") (TriggeredSeconds :type "Float (double-precision)") (InputAction :type "InputAction Object Reference" :default "/Game/Postal2/Blueprint/Core/EnhancedInput/Action/IA_PostalPauseMenu.IA_PostalPauseMenu"))
  (:`Triggered`
    (if (`GameplayStatics.IsGamePaused`)
      (`GameplayStatics.SetGamePaused` false)
      (`WidgetBlueprintLibrary.SetInputMode_GameOnly` self)
      (set `self.bShowMouseCursor` false)
      (bind _pausemenuwidget (`self.PauseMenuWidget`)
        (:`then`
          (`Widget.RemoveFromParent` _pausemenuwidget))
        (:`else`))
      (else
        (`GameplayStatics.SetGamePaused` true)
        (`self.PauseMenuWidget`
          (:`then`
            _)
          (:`else`
            (bind _returnvalue (`|CreateWidget` "/Game/Postal2/Blueprint/Core/Widgets/WBP_MainPauseMenu.WBP_MainPauseMenu_C" self))
            (bind _output_get (set `self.PauseMenuWidget` _returnvalue))))
        (`UserWidget.AddToViewport` _output_get 0)
        (`WidgetBlueprintLibrary.SetInputMode_GameAndUIEx` self _output_get)
        (set `self.bShowMouseCursor` true)))))

(fn `UserConstructionScript`)