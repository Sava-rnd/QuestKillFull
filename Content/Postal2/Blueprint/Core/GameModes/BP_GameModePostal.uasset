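; Game mode for the Postal2 project that respawns the player after death and runs the in-game date and time.
; On restart it binds to the character's death dispatcher; death unpossesses the controller, waits briefly, destroys the character and restarts the player.
; A looping timer, with its interval derived from TimeUnit at construction, advances the clock in ten-second steps, rolls over the calendar and rebuilds the DateTime struct.
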(event `self.K2_OnRestartPlayer`
  (params (NewPlayer :type "Controller Object Reference"))
  ;[0 0 0 0.507] Захват персонажа
  (bind _asbp_base_character (cast `/Game/Postal2/Blueprint/Core/Character/BP_BaseCharacter` (`Controller.K2_GetPawn` NewPlayer)))
  (bind _output_get (set `self.CurrentPlayerCharacter` _asbp_base_character))
  (add `/Game/Postal2/Blueprint/Core/Character/BP_BaseCharacter.OnDeathDispather` _output_get (delegate `OnPlayerDeath`)))

(event `OnPlayerDeath`
  (params (Source :type "/Game/Postal2/Blueprint/Core/Character/BP_BaseCharacter Object Reference"))
  (bind _currentplayercharacter (`self.CurrentPlayerCharacter`))
  (`/Engine/EditorBlueprintResources/StandardMacros.IsValid` _currentplayercharacter
    (:`Is Valid`
      (remove `/Game/Postal2/Blueprint/Core/Character/BP_BaseCharacter.OnDeathDispather` _currentplayercharacter (delegate `OnPlayerDeath`))
      (`Controller.UnPossess` (`GameplayStatics.GetPlayerController` 0))
      (`KismetSystemLibrary.Delay` 2.0)
      (`self.K2_DestroyActor` (`self.CurrentPlayerCharacter`))
      (`self.RestartPlayer` (`GameplayStatics.GetPlayerController` 0)))))

(event `self.ReceiveBeginPlay`
  (`KismetSystemLibrary.DelayUntilNextTick`)
  ;[0 0 0 0.507] Игровое время
  (`KismetSystemLibrary.K2_SetTimer` null "CreateClockwork" (`self.GameSpeed`) true))

(fn `CreateClockwork`
  ;[0 0 0 0.507] Создание часового механизма
  (`self.SetClock`)
  (`self.SetCalendar`)
  (`self.SetDateTime`))

(fn `SetCalendar`
  ;[0 0 0 0.507] Установка даты
  (if (>= (`self.Hours`) 24)
    (set `self.Hours` 0)
    (bind _output_get (set `self.Day` (+ (`self.Day`) 1)))
    (if (> _output_get (`KismetMathLibrary.DaysInMonth` (`self.Year`) (`self.Month`)))
      (set `self.Day` 1)
      (set `self.Month` (+ (`self.Month`) 1))
      (if (> (`self.Month`) 12)
        (set `self.Month` 1)
        (set `self.Year` (+ (`self.Year`) 1)))))
  (return))

(fn `SetClock`
  ;[0 0 0 0.507] Проверка паузы
  (if (!= (`self.TimeUnit`) 0.0)
    ;[0 0 0 0.507] Установка времени
    (set `self.Seconds` (+ (`self.Seconds`) 10))
    (if (>= (`self.Seconds`) 60)
      (set `self.Seconds` 0)
      (set `self.Minutes` (+ (`self.Minutes`) 1))
      (if (>= (`self.Minutes`) 60)
        (set `self.Minutes` 0)
        (set `self.Hours` (+ (`self.Hours`) 1)))))
  (return))

(fn `SetDateTime`
  (set `self.DateTimeStruct` (`KismetMathLibrary.MakeDateTime` (`self.Year`) (`self.Month`) (`self.Day`) (`self.Hours`) (`self.Minutes`) (`self.Seconds`)))
  (return))

(fn `UserConstructionScript`
  ;[0 0 0 0.507] Рассчёт скорости игрового времени
  (set `self.GameSpeed` (/ (/ 1.0 (* (`self.TimeUnit`) 5.0)) 6.0)))