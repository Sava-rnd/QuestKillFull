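; BP_NPCDialogue is an NPC dialogue actor that tells the player character when it is within speaking range.
; Each Tick it tests overlap with BP_SkeletonPlayer and shows or hides SpeakWidget to match.
; While the widget is valid, it messages the player the zone state, plus the NPC's name and icon when overlapping.
; Its FuncIsinSpeakZone event destroys the widget, which stops those updates.
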(event `self.ReceiveTick`
  (params (DeltaSeconds :type "Float (single-precision)"))
  (bind _returnvalue (`GameplayStatics.GetPlayerCharacter` 0))
  (bind _speakwidget (`self.SpeakWidget`))
  (if (`self.IsOverlappingActor` (cast `/Game/Postal2/Blueprint/Core/Character/BP_SkeletonPlayer` (`GameplayStatics.GetPlayerCharacter` 0) :!pure true))
    (set `self.bIsInSpeakZone` true)
    (`/Engine/EditorBlueprintResources/StandardMacros.IsValid` (`self.SpeakWidget`)
      (:`Is Valid`
        (`SceneComponent.SetVisibility` _speakwidget true false)
        (message `/Game/Postal2/Blueprint/Core/Character/Interfaces/BPI_Dialogue.Func_IsInSpeakZone` _returnvalue (`self.bIsInSpeakZone`))
        (message `/Game/Postal2/Blueprint/Core/Character/Interfaces/BPI_Dialogue.Func_ManageWidget` (`GameplayStatics.GetPlayerCharacter` 0) (`self.CharacterName`) (`self.CharacterIcon`))))
    (else
      (set `self.bIsInSpeakZone` false)
      (`/Engine/EditorBlueprintResources/StandardMacros.IsValid` (`self.SpeakWidget`)
        (:`Is Valid`
          (`SceneComponent.SetVisibility` _speakwidget false false)
          (message `/Game/Postal2/Blueprint/Core/Character/Interfaces/BPI_Dialogue.Func_IsInSpeakZone` _returnvalue (`self.bIsInSpeakZone`)))))))

(event `/Game/Postal2/Blueprint/Core/Character/Interfaces/BPI_Dialogue.Func_IsInSpeakZone`
  (params (bIsSpeakZone :type Boolean))
  (bind _speakwidget (`self.SpeakWidget`))
  (`/Engine/EditorBlueprintResources/StandardMacros.IsValid` _speakwidget
    (:`Is Valid`
      (`ActorComponent.K2_DestroyComponent` _speakwidget))))

(fn `UserConstructionScript`)