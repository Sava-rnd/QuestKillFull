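; BP_NPCQuest is a quest NPC Blueprint that reveals floating text when the skeleton player enters its box collision.
; The overlap sets IsActorOverlapping and makes the TextRender visible.
; A short Delay loop then keeps turning the text toward player character 0 using FindLookAtRotation.
; The graph has no exit from this loop and no end-overlap handling to hide the text.
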(event `self.BoxCollision.OnComponentBeginOverlap`
  (params (OverlappedComponent :type "PrimitiveComponent Object Reference") (OtherActor :type "Actor Object Reference") (OtherComp :type "PrimitiveComponent Object Reference") (OtherBodyIndex :type Integer) (bFromSweep :type Boolean) (SweepResult :type "HitResult Structure (by ref)"))
  (bind _textrender (`self.TextRender`))
  (cast `/Game/Postal2/Blueprint/Core/Character/BP_SkeletonPlayer` OtherActor)
  (set `self.bIsActorOverlapping?` true)
  (`SceneComponent.SetVisibility` _textrender true false)
  (`SceneComponent.K2_SetWorldRotation` (`self.TextRender`) (`KismetMathLibrary.FindLookAtRotation` (`SceneComponent.K2_GetComponentLocation` _textrender) (`self.K2_GetActorLocation` (`GameplayStatics.GetPlayerCharacter` 0))) false false :!label _label)
  (`KismetSystemLibrary.Delay` 0.01)
  (goto _label))

(fn `UserConstructionScript`)