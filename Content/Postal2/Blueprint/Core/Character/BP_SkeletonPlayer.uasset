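; BP_SkeletonPlayer is the player character, handling interaction, physical animation and death.
; The interact input fires several independent paths: camera traces for quest and cleaver interfaces, look-at objective reporting, and NPC dialogue with a camera blend inside speak zones.
; Tick traces for look-at targets, refreshes movement gameplay tags and moves the actor to the mesh while ragdolled.
; Physical animation starts at BeginPlay; death switches to ragdoll and disables capsule collision.
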(event `EnhancedInput|/Game/Postal2/Blueprint/Core/EnhancedInput/Action/IA_PostalInteract`
  (params (ActionValue :type Boolean) (ElapsedSeconds :type "Float (double-precision)") (TriggeredSeconds :type "Float (double-precision)") (InputAction :type "InputAction Object Reference" :default "/Game/Postal2/Blueprint/Core/EnhancedInput/Action/IA_PostalInteract.IA_PostalInteract"))
  (:`Started`
    (bind _hitactor (`self.LineTraceToCamera`))
    (`self.BranchToInteractQuest` _hitactor _hitactor)))

(event `self.ReceiveBeginPlay`
  ;[0 0 0 0.507] Включение физики
  (`parent.ReceiveBeginPlay`)
  (`self.GetDialogueCamera`)
  (`self.EnableToPA`))

(event `self.ReceiveTick`
  (params (DeltaSeconds :type "Float (single-precision)"))
  (`parent.ReceiveTick` DeltaSeconds)
  (`self.InteractTrace`)
  (`self.AssemblingMovement`))

(event `self.OnDeath`
  ;[0 0 0 0.507] Обработка смерти
  (`parent.OnDeath`)
  (`self.ToInDeath`))

(event `/Game/Postal2/Blueprint/Core/Character/Interfaces/BPI_Dialogue.Func_IsInSpeakZone`
  (params (bIsSpeakZone :type Boolean))
  (set `self.Is Speak Zone` bIsSpeakZone))

(event `EnhancedInput|/Game/Postal2/Blueprint/Core/EnhancedInput/Action/IA_PostalInteract`
  (params (ActionValue :type Boolean) (ElapsedSeconds :type "Float (double-precision)") (TriggeredSeconds :type "Float (double-precision)") (InputAction :type "InputAction Object Reference" :default "/Game/Postal2/Blueprint/Core/EnhancedInput/Action/IA_PostalInteract.IA_PostalInteract"))
  (:`Started`
    (if (`self.Is Speak Zone`)
      (bind _returnvalue (`GameplayStatics.GetActorOfClass` "/Game/Postal2/Blueprint/Core/Character/BP_NPCDialogue.BP_NPCDialogue_C"))
      (message `/Game/Postal2/Blueprint/Core/Character/Interfaces/BPI_Dialogue.Func_IsInSpeakZone` _returnvalue (`self.Is Speak Zone`))
      (`PlayerController.SetViewTargetWithBlend` (`GameplayStatics.GetPlayerController` 0) (`self.BP_DialogueCamera`) 1.0 "VTBlend_Linear" 0.0 false)
      (`self.DisableInput` self (`GameplayStatics.GetPlayerController` 0))
      (message `/Game/Postal2/Blueprint/Core/Character/Interfaces/BPI_Dialogue.Func_ManageWidget` (`self.BPC_Dialogue`) (`self.Character Name`) (`self.Character Icon`)))))

(event `/Game/Postal2/Blueprint/Core/Character/Interfaces/BPI_Dialogue.Func_ManageWidget`
  (params (CharacterName :type Text) (CharacterIcon :type "Texture2D Object Reference"))
  (set `self.Character Name` CharacterName)
  (set `self.Character Icon` CharacterIcon))

(event `EnhancedInput|/Game/Postal2/Blueprint/Core/EnhancedInput/Action/IA_PostalInteract`
  (params (ActionValue :type Boolean) (ElapsedSeconds :type "Float (double-precision)") (TriggeredSeconds :type "Float (double-precision)") (InputAction :type "InputAction Object Reference" :default "/Game/Postal2/Blueprint/Core/EnhancedInput/Action/IA_PostalInteract.IA_PostalInteract"))
  ;[0 0 0 0.507] Взять квест
  (:`Started`
    (set `self.bIsReadyForQuest` true))
  (:`Completed`
    (set `self.bIsReadyForQuest` false)))

(event `EnhancedInput|/Game/Postal2/Blueprint/Core/EnhancedInput/Action/IA_PostalInteract`
  (params (ActionValue :type Boolean) (ElapsedSeconds :type "Float (double-precision)") (TriggeredSeconds :type "Float (double-precision)") (InputAction :type "InputAction Object Reference" :default "/Game/Postal2/Blueprint/Core/EnhancedInput/Action/IA_PostalInteract.IA_PostalInteract"))
  (:`Started`
    (bind _lookatactor (`self.LookAtActor`)
      (:`then`
        (bind _objectiveid (message `/Game/Postal2/Blueprint/Core/GameSystem/QuestSystem/IInteractionInterface.InteractionWith` _lookatactor))
        (`self.OnObjectiveIDCalled` _objectiveid 1))
      (:`else`))))

(event `EnhancedInput|/Game/Postal2/Blueprint/Core/EnhancedInput/Action/IA_PostalInteract`
  (params (ActionValue :type Boolean) (ElapsedSeconds :type "Float (double-precision)") (TriggeredSeconds :type "Float (double-precision)") (InputAction :type "InputAction Object Reference" :default "/Game/Postal2/Blueprint/Core/EnhancedInput/Action/IA_PostalInteract.IA_PostalInteract"))
  (bind _camera (`self.Camera`))
  (bind _returnvalue (`SceneComponent.K2_GetComponentLocation` _camera))
  (:`Started`
    (bind (_outhit _returnvalue_2) (`KismetSystemLibrary.LineTraceSingle` :`Start` _returnvalue :`End` (+ _returnvalue (* (`SceneComponent.GetForwardVector` _camera) 300.0)) :`TraceChannel` "TraceTypeQuery1" :`DrawDebugType` "ForDuration"))
    (if _returnvalue_2
      (bind (_bblockinghit _binitialoverlap _time _distance _location _impactpoint _normal _impactnormal _physmat _hitactor) (`GameplayStatics.BreakHitResult` _outhit))
      (if _bblockinghit
        (if (`KismetSystemLibrary.DoesImplementInterface` _hitactor "/Game/Postal2/Blueprint/Core/InteractionCleaver/BPI_InteractionCleaver.BPI_InteractionCleaver_C")
          (message `/Game/Postal2/Blueprint/Core/InteractionCleaver/BPI_InteractionCleaver.Interact` _hitactor))))))

(fn `DisablePA`
  (`PhysicalAnimationComponent.SetSkeletalMeshComponent` (`self.PhysicalAnimation`) (`self.Mesh`)))

(fn `DisableRagdoll`
  (params (SnapTransform :type "Transform Structure (by ref)"))
  (`PrimitiveComponent.SetSimulatePhysics` (`self.Mesh`) false)
  (`PrimitiveComponent.SetCollisionProfileName` (`self.Mesh`) "CharacterMesh" true)
  (`SceneComponent.K2_AttachToComponent` (`self.Mesh`) (`self.CapsuleComponent`) "None" "SnapToTarget" "SnapToTarget" "SnapToTarget" true)
  (`SceneComponent.K2_SetRelativeTransform` (`self.Mesh`) SnapTransform false false))

(fn `EnablePA`
  (params (BodyName :type Name :default "none"))
  (`PhysicalAnimationComponent.SetSkeletalMeshComponent` (`self.PhysicalAnimation`) (`self.Mesh`))
  (`PhysicalAnimationComponent.ApplyPhysicalAnimationSettingsBelow` (`self.PhysicalAnimation`) BodyName (make `PhysicalAnimationData` false 1000.0 100.0 1000.0 100.0) true)
  (`SkeletalMeshComponent.SetAllBodiesBelowSimulatePhysics` (`self.Mesh`) BodyName true true)
  (`PrimitiveComponent.SetCollisionProfileName` (`self.Mesh`) "Ragdoll" true))

(fn `EnableRagdoll`
  (params (InBoneName :type Name))
  (returns (InitialRelativeTransform :type "Transform Structure"))
  (locals (InitialTransform :type "Transform Structure"))
  (set `local.InitialTransform` (`SceneComponent.GetRelativeTransform` (`self.Mesh`)))
  (`PrimitiveComponent.SetCollisionProfileName` (`self.Mesh`) "Ragdoll" true)
  (`SkeletalMeshComponent.SetAllBodiesBelowSimulatePhysics` (`self.Mesh`) InBoneName true true)
  (return (`local.InitialTransform`)))

(fn `InteractTrace`
  (bind _returnvalue (`GameplayStatics.GetPlayerCameraManager` 0))
  (bind _returnvalue_2 (`self.K2_GetActorLocation` _returnvalue))
  (bind (_outhit _returnvalue_3) (`KismetSystemLibrary.LineTraceSingle` _returnvalue_2 (+ _returnvalue_2 (* (`self.GetActorForwardVector` _returnvalue) 600.0)) "TraceTypeQuery1"))
  (if _returnvalue_3
    (bind (_bblockinghit _binitialoverlap _time _distance _location _impactpoint _normal _impactnormal _physmat _hitactor) (`GameplayStatics.BreakHitResult` _outhit))
    (if (`KismetSystemLibrary.DoesImplementInterface` _hitactor "/Game/Postal2/Blueprint/Core/GameSystem/QuestSystem/IInteractionInterface.IInteractionInterface_C")
      (bind _output_get (set `self.LookAtActor` _hitactor))
      (message `/Game/Postal2/Blueprint/Core/GameSystem/QuestSystem/IInteractionInterface.LookAt` _output_get)
      (else
        (set `self.LookAtActor` null)))
    (else
      (set `self.LookAtActor` null))))

(fn `UserConstructionScript`
  (`parent.UserConstructionScript`)
  (`SceneComponent.K2_AttachToComponent` (`self.MeleeHitCollision`) (`self.Mesh`) "Melee_Socket" "SnapToTarget" "SnapToTarget" "SnapToTarget" true))