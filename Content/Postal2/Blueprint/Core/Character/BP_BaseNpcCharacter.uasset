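; Base NPC character Blueprint that handles death, ragdoll physics and physical animation.
; On death it flags the NPC as dead, ragdolls the mesh from a root bone, disables capsule collision and destroys the actor after a short delay.
; Helper functions drive physical animation below a chosen bone, toggle ragdoll with the mesh's relative transform returned for re-snapping to the capsule, and set walk speed.
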(event `self.OnDeath`
  ;[0 0 0 0.507] Обработка смерти
  (`parent.OnDeath`)
  (set `self.bIsDeath` true)
  (`self.DisablePA`)
  (`self.EnableRagdoll` (`self.RootRagdollBone`))
  (`PrimitiveComponent.SetCollisionEnabled` (`self.CapsuleComponent`) "NoCollision")
  (set `PrimitiveComponent.bGenerateOverlapEvents` false (`self.CapsuleComponent`))
  (`KismetSystemLibrary.Delay` 3.0)
  (`self.K2_DestroyActor`))

(fn `DisablePA`
  (`PhysicalAnimationComponent.SetSkeletalMeshComponent` (`self.PhysicalAnimation`) (`self.Mesh`)))

(fn `DisableRagdoll`
  (params (SnapTransform :type "Transform Structure (by ref)"))
  (`PrimitiveComponent.SetSimulatePhysics` (`self.Mesh`) false)
  (`PrimitiveComponent.SetCollisionProfileName` (`self.Mesh`) "CharacterMesh" true)
  (`SceneComponent.K2_AttachToComponent` (`self.Mesh`) (`self.CapsuleComponent`) "None" "SnapToTarget" "SnapToTarget" "SnapToTarget" true)
  (`SceneComponent.K2_SetRelativeTransform` (`self.Mesh`) SnapTransform false false))

(fn `EnablePA`
  (params (BodyName :type Name :default "none"))
  (`PhysicalAnimationComponent.SetSkeletalMeshComponent` (`self.PhysicalAnimation`) (`self.Mesh`))
  (`PhysicalAnimationComponent.ApplyPhysicalAnimationSettingsBelow` (`self.PhysicalAnimation`) BodyName (make `PhysicalAnimationData` false 1000.0 100.0 1000.0 100.0) true)
  (`SkeletalMeshComponent.SetAllBodiesBelowSimulatePhysics` (`self.Mesh`) BodyName true true)
  (`PrimitiveComponent.SetCollisionProfileName` (`self.Mesh`) "Ragdoll" true))

(fn `EnableRagdoll`
  (params (InBoneName :type Name))
  (returns (InitialRelativeTransform :type "Transform Structure"))
  (locals (InitialTransform :type "Transform Structure"))
  (set `self.InitialMeshRelativeTransform` (`SceneComponent.GetRelativeTransform` (`self.Mesh`)))
  (`PrimitiveComponent.SetCollisionProfileName` (`self.Mesh`) "Ragdoll" true)
  (`SkeletalMeshComponent.SetAllBodiesBelowSimulatePhysics` (`self.Mesh`) InBoneName true true)
  (return (`self.InitialMeshRelativeTransform`)))

(fn `UpdateWalkSpeed`
  (params (`Max Walk Speed` :type "Float (single-precision)"))
  (set `CharacterMovementComponent.MaxWalkSpeed` `Max Walk Speed` (`self.CharacterMovement`)))

(fn `UserConstructionScript`
  (`parent.UserConstructionScript`))