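; Base character Blueprint built on the Gameplay Ability System, handling melee hit detection, health and death.
; A melee collision overlap is confirmed with a multi-object line trace, then sends a hit gameplay event with target data back to the attacker.
; On BeginPlay it binds itself to the health bar widget and watches attribute changes, applying a death effect and calling the death dispatcher when health reaches zero.
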(event `self.MeleeHitCollision.OnComponentBeginOverlap`
  (params (OverlappedComponent :type "PrimitiveComponent Object Reference") (OtherActor :type "Actor Object Reference") (OtherComp :type "PrimitiveComponent Object Reference") (OtherBodyIndex :type Integer) (bFromSweep :type Boolean) (SweepResult :type "HitResult Structure (by ref)"))
  (if (!= OtherActor self)
    (bind _asbp_base_character (cast `/Game/Postal2/Blueprint/Core/Character/BP_BaseCharacter` OtherActor))
    (bind _outhits (`KismetSystemLibrary.LineTraceMultiForObjects` (`SceneComponent.K2_GetComponentLocation` (`self.MeleeHitCollision`)) (`self.K2_GetActorLocation` _asbp_base_character) (`|MakeArray` "ObjectTypeQuery3" "ObjectTypeQuery2" :!type "EObjectTypeQuery Enum") false (`|MakeArray` self :!type "Actor Object Reference")))
    (for _array_element _outhits
      (if (== (`.HitActor` (`GameplayStatics.BreakHitResult` _array_element)) _asbp_base_character)
        (`AbilitySystemBlueprintLibrary.SendGameplayEventToActor` self (struct :`TagName` "Event.Ability.MeleeAttack.Hit") (make `GameplayEventData` (struct) null null null null (struct) (struct) (struct) 0.0 (`AbilitySystemBlueprintLibrary.AbilityTargetDataFromHitResult` _array_element)))
        (break)))))

(event `self.ReceiveBeginPlay`
  (`parent.ReceiveBeginPlay`)
  (`|ExecutionSequence`
    (:`then_0`
      (`self.FillToHealth`))
    (:`then_1`
      (`self.HealthAndDeathCheck`))))

(event `OnDeath`
  (`AbilitySystemComponent.BP_ApplyGameplayEffectToSelf` :`self` (`self.AbilitySystem`) :`GameplayEffectClass` "/Game/Postal2/Blueprint/Core/GameSystem/GameAbilitiеs/PassiveEffect/GE_Death.GE_Death_C")
  (`self.OnDeathDispather` self))

(fn `GetHealth`
  (returns (Result :type "Float (double-precision)"))
  (return (`/Game/Postal2/Blueprint/Core/GameSystem/BP_AttributesComponents.GetHealth` (`self.Attributes`))))

(fn `GetIsInStealth`
  (returns (Result :type Boolean))
  (return (`/Game/Postal2/Blueprint/Core/GameSystem/BP_AttributesComponents.GetIsInStealth` (`self.Attributes`))))

(fn `GetSneak`
  (returns (Result :type "Float (double-precision)"))
  (return (`/Game/Postal2/Blueprint/Core/GameSystem/BP_AttributesComponents.GetSneak` (`self.Attributes`))))

(fn `UserConstructionScript`)