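; Sprint gameplay ability that raises the character's walk speed while input is held and cost can be paid.
; Activation removes the stamina regen effect and commits the ability, then a 0.1-second delay loop repeatedly commits the cost and sets sprint speed.
; Input release or a failed cost restores normal speed and ends the ability.
; On end, it starts a timer with no visible callback and immediately reapplies stamina regen.
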(event `self.K2_ActivateAbility`
  (bind _asbp_base_character (cast `/Game/Postal2/Blueprint/Core/Character/BP_BaseCharacter` (`self.GetAvatarActorFromActorInfo`))
    (:`then`
      (bind _output_get (set `self.AvatarCharacter` _asbp_base_character))
      (`AbilitySystemComponent.RemoveActiveGameplayEffectBySourceEffect` (`/Game/Postal2/Blueprint/Core/Character/BP_BaseCharacter.AbilitySystem` _output_get) "/Game/Postal2/Blueprint/Core/GameSystem/GameAbilitiеs/PassiveEffect/GE_StaminaRegen.GE_StaminaRegen_C" null -1)
      (bind _returnvalue (`self.K2_CommitAbility`))
      (if _returnvalue
        (`AbilityTask_WaitInputRelease.WaitInputRelease` false
          (:`then`
            (`AbilityTask_WaitDelay.WaitDelay` 0.1 :!label _label
              (:`OnFinish`
                (bind _returnvalue_2 (`self.K2_CommitAbilityCost` false))
                (if _returnvalue_2
                  (set `CharacterMovementComponent.MaxWalkSpeed` 600.0 (`Character.CharacterMovement` (`self.AvatarCharacter`)))
                  (goto _label)
                  (else
                    _)))))
          (:`OnRelease`
            _))
        (set `CharacterMovementComponent.MaxWalkSpeed` 300.0 (`Character.CharacterMovement` (`self.AvatarCharacter`)))
        (`self.K2_EndAbility`)
        (else
          (`self.K2_CancelAbility`))))
    (:`CastFailed`
      (`self.K2_CancelAbility`))))

(event `self.K2_OnEndAbility`
  (params (bWasCancelled :type Boolean))
  (`KismetSystemLibrary.K2_SetTimerDelegate` :`Time` 3.0)
  (bind _returnvalue (`AbilitySystemComponent.BP_ApplyGameplayEffectToSelf` :`self` (`/Game/Postal2/Blueprint/Core/Character/BP_BaseCharacter.AbilitySystem` (`self.AvatarCharacter`)) :`GameplayEffectClass` "/Game/Postal2/Blueprint/Core/GameSystem/GameAbilitiеs/PassiveEffect/GE_StaminaRegen.GE_StaminaRegen_C"))
  (set `self.HandleStamina` _returnvalue))