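; GA_Stealth is a hold-to-use gameplay ability that puts a BP_BaseCharacter avatar into stealth.
; On activation it crouches the character, applies GE_Stealth to the owner and stores the effect handle, or cancels if the avatar is invalid.
; Releasing the input ends the ability, which uncrouches and removes the effect by handle.
; This cleanup is skipped when the ability is cancelled.
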(event `self.K2_ActivateAbility`
  (bind _returnvalue (`self.GetAvatarActorFromActorInfo`))
  (`/Engine/EditorBlueprintResources/StandardMacros.IsValid` _returnvalue
    (:`Is Valid`
      (bind _asbp_base_character (cast `/Game/Postal2/Blueprint/Core/Character/BP_BaseCharacter` _returnvalue)
        (:`then`
          (bind _output_get (set `self.AvatarCharacter` _asbp_base_character))
          (`Character.Crouch` _output_get)
          (bind _returnvalue_2 (`self.BP_ApplyGameplayEffectToOwner` "/Game/Postal2/Blueprint/Core/GameSystem/GameAbilitiеs/Stealth/GE_Stealth.GE_Stealth_C"))
          (set `self.AppliedEffect` _returnvalue_2)
          (`AbilityTask_WaitInputRelease.WaitInputRelease` false
            (:`OnRelease`
              (`self.K2_EndAbility`))))
        (:`CastFailed`
          (`self.K2_CancelAbility`))))
    (:`Is Not Valid`
      (`self.K2_CancelAbility`))))

(event `self.K2_OnEndAbility`
  (params (bWasCancelled :type Boolean))
  (if (not bWasCancelled)
    (`Character.UnCrouch` (`self.AvatarCharacter`))
    (`self.BP_RemoveGameplayEffectFromOwnerWithHandle` (`self.AppliedEffect`))))