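; BP_Turret is an automated turret that patrols and fires on characters it detects.
; A timeline sweeps the gun back and forth across 180 degrees while Tick runs a Patrol/Shoot state machine driven by a barrel sphere trace.
; In Shoot, the gun's yaw tracks the player and a looping timer fires line traces, playing explosion effects on hits and applying GAS damage to BP_BaseCharacter targets.
; Losing the target clears the timer and resumes patrol.
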(event `StopPatrol`
  (bind (_direction _rotatetrack) (`Timeline|Rotator` :!via `Stop` :!label _label)
    (:`Update`
      (`SceneComponent.K2_SetWorldRotation` (`self.Gun`) (`KismetMathLibrary.RLerp` (`self.CurrentRotation`) (`self.TargetRotation`) _rotatetrack) false false))
    (:`Finished`
      (switch `ETimelineDirection` (`self.DirectionMove`)
        (:`Forward`
          (set `self.DirectionMove` "Backward")
          (set `self.TargetRotation` (`self.StartRotation`))
          (set `self.CurrentRotation` (`self.EndRotation`)))
        (:`Backward`
          (set `self.DirectionMove` "Forward")
          (set `self.TargetRotation` (`self.EndRotation`))
          (set `self.CurrentRotation` (`self.StartRotation`))))
      (`self.StartPatrol`))))

(event `self.ReceiveBeginPlay`
  (bind _output_get (set `self.StartRotation` (`SceneComponent.K2_GetComponentRotation` (`self.Gun`))))
  (set `self.EndRotation` (`KismetMathLibrary.MakeRotator` (.roll _output_get) (.pitch _output_get) (+ (.yaw _output_get) 180.0)))
  (set `self.CurrentRotation` (`self.CurrentRotation`))
  (set `self.TargetRotation` (`self.EndRotation`))
  (`self.StartPatrol`))

(event `StartPatrol`
  (goto _label :!via `PlayFromStart`))

(event `StartShoot`
  (bind _returnvalue (`KismetSystemLibrary.K2_SetTimerDelegate` (delegate `CallShootFunc`) 1.0 true))
  (set `self.TH_Shoot` _returnvalue))

(event `CallShootFunc`
  (bind _bisshoot (`self.PlayerShoot`))
  (if _bisshoot
    _))

(event `self.ReceiveTick`
  (params (DeltaSeconds :type "Float (single-precision)"))
  (bind _gun (`self.Gun`))
  (bind (_returnvalue_roll _returnvalue_pitch _returnvalue_yaw) (`KismetMathLibrary.BreakRotator` (`SceneComponent.K2_GetComponentRotation` _gun)))
  (bind (_returnvalue_roll_2 _returnvalue_pitch_2 _returnvalue_yaw_2) (`KismetMathLibrary.BreakRotator` (`KismetMathLibrary.FindLookAtRotation` (`SceneComponent.K2_GetComponentLocation` (`self.Gun`)) (`self.K2_GetActorLocation` (`GameplayStatics.GetPlayerCharacter` 0)))))
  (`/Engine/EditorBlueprintResources/StandardMacros.IsValid` (`GameplayStatics.GetPlayerPawn` 0)
    (:`Is Valid`
      (switch `/Game/Postal2/Blueprint/Core/Enums/E_TurretStates` (`self.CurrentState`)
        (:`NewEnumerator0`
          (bind _bisplayerfind (`self.PlayerSearch`))
          (if _bisplayerfind
            (`self.StopPatrol`)
            (set `self.CurrentState` "NewEnumerator1")))
        (:`NewEnumerator1`
          (`SceneComponent.K2_SetWorldRotation` _gun (`KismetMathLibrary.RInterpTo` (`KismetMathLibrary.MakeRotator` _returnvalue_roll _returnvalue_pitch _returnvalue_yaw) (`KismetMathLibrary.MakeRotator` _returnvalue_roll _returnvalue_pitch (- _returnvalue_yaw_2 90.0)) (`GameplayStatics.GetWorldDeltaSeconds`)) false false)
          (`|ExecutionSequence`
            (:`then_0`
              (if (not (`self.bIsStartShoot`))
                (`self.StartShoot`)
                (set `self.bIsStartShoot` true)))
            (:`then_1`
              (bind _bisplayerfind_2 (`self.PlayerSearch`))
              (if (not _bisplayerfind_2)
                (`KismetSystemLibrary.K2_ClearAndInvalidateTimerHandle` (`self.TH_Shoot`))
                (set `self.bIsStartShoot` false)
                (set `self.CurrentState` "NewEnumerator0")
                (set `self.TargetRotation` (`self.EndRotation`))
                (set `self.CurrentRotation` (`SceneComponent.K2_GetComponentRotation` (`self.Gun`)))
                (set `self.DirectionMove` "Forward")
                (`self.StartPatrol`)))))))))

(fn `PlayerSearch`
  (returns (bIsPlayerFind :type Boolean))
  (bind _barrel (`self.Barrel`))
  (bind _returnvalue (`SceneComponent.K2_GetComponentLocation` _barrel))
  (bind (_outhit _returnvalue_2) (`KismetSystemLibrary.SphereTraceSingle` _returnvalue (+ _returnvalue (* (`SceneComponent.GetForwardVector` _barrel) (`self.SearchDistance`))) 10.0 "TraceTypeQuery3"))
  (if _returnvalue_2
    (cast `/Game/Postal2/Blueprint/Core/Character/BP_BaseCharacter` (`.HitActor` (`GameplayStatics.BreakHitResult` _outhit))
      (:`then`
        (return true))
      (:`CastFailed`
        (return false)))
    (else
      (return false))))

(fn `PlayerShoot`
  (returns (bIsShoot :type Boolean))
  (locals (DamageEffectContext :type "GameplayEffectContextHandle Structure"))
  (bind _barrel (`self.Barrel`))
  (bind _returnvalue (`SceneComponent.K2_GetComponentLocation` _barrel))
  (bind (_outhit _returnvalue_2) (`KismetSystemLibrary.LineTraceSingle` _returnvalue (+ _returnvalue (* (`SceneComponent.GetForwardVector` _barrel) (`self.ShootDistance`))) "TraceTypeQuery3"))
  (if _returnvalue_2
    (`|ExecutionSequence`
      (:`then_0`
        (`GameplayStatics.PlaySoundAtLocation` "/Game/StarterContent/Audio/Explosion_Cue.Explosion_Cue" (`SceneComponent.K2_GetComponentLocation` (`self.Barrel`)) (struct) 1.0 1.0 0.0 null null null null)
        (`GameplayStatics.SpawnEmitterAttached` "/Game/StarterContent/Particles/P_Explosion.P_Explosion" (`self.Barrel`) "None" (0.0 0.0 0.0) (struct) (0.2 0.2 0.2)))
      (:`then_1`
        (bind _asbp_base_character (cast `/Game/Postal2/Blueprint/Core/Character/BP_BaseCharacter` (`.HitActor` (`GameplayStatics.BreakHitResult` _outhit)))
          (:`then`
            (bind _output_get (set `local.DamageEffectContext` (`AbilitySystemComponent.MakeEffectContext` (`self.AbilitySystem`))))
            (`AbilitySystemBlueprintLibrary.EffectContextAddHitResult` _output_get _outhit)
            (`AbilitySystemComponent.BP_ApplyGameplayEffectToTarget` (`self.AbilitySystem`) "/Game/Postal2/Blueprint/Core/GameSystem/GameAbilitiеs/MeleeAttack/GE_MeleeAttack_Damage.GE_MeleeAttack_Damage_C" (`AbilitySystemBlueprintLibrary.GetAbilitySystemComponent` _asbp_base_character) 0.0 (`local.DamageEffectContext`))
            (return true))
          (:`CastFailed`
            (return false)))))
    (else
      (return false))))

(fn `UserConstructionScript`)