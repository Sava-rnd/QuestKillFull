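; AI controller for a skeleton guard that runs its behavior tree on possess and feeds it sight and hearing perception through the Blackboard.
; Sight tracks only the current player, setting the enemy and line-of-sight keys, or clearing them when sight fails or stealth hides the player.
; Stealth hides the player beyond a distance that shrinks as their sneak value rises.
; Hearing stores a location to investigate when the sensed character has a walking tag.
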(event `self.ReceivePossess`
  (params (PossessedPawn :type "Pawn Object Reference"))
  (`self.RunBehaviorTree` "/Game/Postal2/Blueprint/Core/ArtificialIntelligence/BT_SkeletonGuardTree.BT_SkeletonGuardTree"))

(event `self.AIPerception.OnTargetPerceptionUpdated`
  (params (Actor :type "Actor Object Reference") (Stimulus :type "AIStimulus Structure"))
  (bind _returnvalue (`AIPerceptionSystem.GetSenseClassForStimulus` Stimulus))
  (`|ExecutionSequence`
    (:`then_0`
      (if (== _returnvalue "/Script/AIModule.AISense_Sight")
        (`self.HandleSilghtSense` Actor Stimulus)))
    (:`then_1`
      (if (== _returnvalue "/Script/AIModule.AISense_Hearing")
        (`self.HandleHearingSense` Actor Stimulus)))))

(fn `HandleHearingSense`
  (params (Actor :type "Actor Object Reference") (Stimulus :type "AIStimulus Structure"))
  (bind (_age _expirationage _strength _stimuluslocation _receiverlocation _tag _bsuccessfullysensed) (break `AIStimulus` (`local.Stimulus`)))
  (bind _asbp_base_character (cast `/Game/Postal2/Blueprint/Core/Character/BP_BaseCharacter` Actor))
  (if (and (`BlueprintGameplayTagLibrary.HasTag` (`/Game/Postal2/Blueprint/Core/Character/BP_BaseCharacter.GameplayTags` _asbp_base_character) (struct :`TagName` "Status.Character.Movement.Walking")) _bsuccessfullysensed)
    (`BlackboardComponent.SetValueAsVector` (`self.Blackboard`) (`self.LocationToInvestigateKey`) _stimuluslocation)))

(fn `HandleSilghtSense`
  (params (Actor :type "Actor Object Reference") (Stimulus :type "AIStimulus Structure"))
  (bind (_age _expirationage _strength _stimuluslocation _receiverlocation) (break `AIStimulus` (`local.Stimulus`)))
  (bind _asbp_base_character (cast `/Game/Postal2/Blueprint/Core/Character/BP_BaseCharacter` Actor))
  (if (`BlueprintGameplayTagLibrary.HasTag` (`/Game/Postal2/Blueprint/Core/Character/BP_BaseCharacter.GameplayTags` _asbp_base_character) (struct :`TagName` "Status.Character.Player.CurrentPlayer"))
    (bind _result (message `/Game/Postal2/Blueprint/Core/Character/Interfaces/BPI_CharacterHelper.GetSneak` _asbp_base_character))
    (if (and (`.bSuccessfullySensed` (break `AIStimulus` (`local.Stimulus`))) (not (and (`GameplayTagAssetInterface.HasMatchingGameplayTag` (`AbilitySystemBlueprintLibrary.GetAbilitySystemComponent` _asbp_base_character) (struct :`TagName` "Status.Character.InStealth")) (> (`KismetMathLibrary.Vector_Distance` _stimuluslocation _receiverlocation) (* (- 1.0 _result) 1000.0)))))
      (`BlackboardComponent.SetValueAsObject` (`self.Blackboard`) (`self.EnemyActorKey`) (`local.Actor`))
      (`BlackboardComponent.SetValueAsBool` (`self.Blackboard`) (`self.HasLineOfSightKey`) true)
      (else
        (`BlackboardComponent.ClearValue` (`self.Blackboard`) (`self.EnemyActorKey`))
        (`BlackboardComponent.ClearValue` (`self.Blackboard`) (`self.HasLineOfSightKey`))))))

(fn `UserConstructionScript`)