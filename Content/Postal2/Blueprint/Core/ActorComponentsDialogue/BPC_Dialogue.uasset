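; BPC_Dialogue is an actor component that starts NPC dialogue through a UI widget and a behavior tree.
; On BeginPlay it caches the first AIC_NPC_Dialogue controller found in the level.
; FuncManageWidget creates WBP_Dialogue with the given name and icon, shows it, and switches input to game and UI with a visible cursor.
; It then runs the behavior tree on that controller and passes the widget through the Blackboard.
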(event `/Game/Postal2/Blueprint/Core/Character/Interfaces/BPI_Dialogue.Func_ManageWidget`
  (params (CharacterName :type Text) (CharacterIcon :type "Texture2D Object Reference"))
  (bind _returnvalue (`GameplayStatics.GetPlayerController` 0))
  (bind _returnvalue_2 (`|CreateWidget` "/Game/Postal2/Blueprint/Core/Widgets/WidgetSubMenu/WBP_Dialogue.WBP_Dialogue_C" null CharacterName CharacterIcon))
  (bind _output_get (set `self.WBP_Dialogue` _returnvalue_2))
  (`UserWidget.AddToViewport` _output_get 0)
  (`WidgetBlueprintLibrary.SetInputMode_GameAndUIEx` _returnvalue (`self.WBP_Dialogue`))
  (set `PlayerController.bShowMouseCursor` true _returnvalue)
  (`AIController.RunBehaviorTree` (`self.AIC_NPC_Controller`) (`self.BTAsset`))
  (`BlackboardComponent.SetValueAsObject` (`AIController.Blackboard` (`self.AIC_NPC_Controller`)) (`self.WBP_DialogueKey`) (`self.WBP_Dialogue`)))

(event `self.ReceiveBeginPlay`
  (bind _returnvalue (`GameplayStatics.GetActorOfClass` "/Game/Postal2/Blueprint/Core/AI/AIC_NPC_Dialogue.AIC_NPC_Dialogue_C"))
  (set `self.AIC_NPC_Controller` _returnvalue))