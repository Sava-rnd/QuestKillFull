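; BPC_QuestDialogue is a dialogue component that starts a quest conversation with a BP_NPCQuest NPC.
; Every tick it looks up that NPC with GetActorOfClass and checks its overlap flag and the player's IsReadyForQuest flag.
; When both are true, a DoOnce gate spawns an AIC_QuestDialogue controller, which creates the dialogue UI and runs the assigned behavior tree to drive the dialogue.
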(event `self.ReceiveTick`
  (params (DeltaSeconds :type "Float (single-precision)"))
  (bind _returnvalue (`GameplayStatics.GetActorOfClass` "/Game/Postal2/Blueprint/Core/Character/BP_NPCQuest.BP_NPCQuest_C"))
  (if (and (`/Game/Postal2/Blueprint/Core/Character/BP_NPCQuest.bIsActorOverlapping?` _returnvalue) (`/Game/Postal2/Blueprint/Core/Character/BP_SkeletonPlayer.bIsReadyForQuest` (cast `/Game/Postal2/Blueprint/Core/Character/BP_SkeletonPlayer` (`GameplayStatics.GetPlayerCharacter` 0) :!pure true)))
    (`/Engine/EditorBlueprintResources/StandardMacros.DoOnce` false
      (:`Completed`
        (bind _returnvalue_2 (`|SpawnActorFromClass` "/Game/Postal2/Blueprint/Core/AI/AIC_QuestDialogue.AIC_QuestDialogue_C" (`KismetMathLibrary.MakeTransform` (0.0 0.0 0.0)) "Undefined" "MultiplyWithRoot" null null))
        (bind _output_get (set `self.AIC_QuestDialogue` _returnvalue_2))
        (`/Game/Postal2/Blueprint/Core/AI/AIC_QuestDialogue.CreateDialogueUI` _output_get)
        (`AIController.RunBehaviorTree` _output_get (`self.BTAsset`))))))