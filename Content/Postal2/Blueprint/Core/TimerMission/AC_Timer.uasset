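; Timed kill-mission actor: interacting starts an hours/minutes/seconds countdown and shows the WG_Timer widget.
; Tick decrements the clock by one second per call; at zero the widget shows complete or failed, with failure resetting the time.
; A looping one-second timer polls the death flag of the BP_BaseNpcCharacter found at BeginPlay.
; Once that NPC dies during the mission, it marks completion and opens TownShops after a short delay.
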(event `self.ReceiveBeginPlay`
  (bind _returnvalue (`GameplayStatics.GetActorOfClass` "/Game/Postal2/Blueprint/Core/Character/BP_BaseNpcCharacter.BP_BaseNpcCharacter_C"))
  (set `self.BasePlayerGuard` _returnvalue)
  (`self.SetActorTickEnabled` false)
  (bind _output_get (set `self.Seconds_0` (`KismetMathLibrary.Clamp` (`self.Seconds`) 0 59)))
  (set `self.Seconds` _output_get)
  (bind _output_get_2 (set `self.Minutes_0` (`KismetMathLibrary.Clamp` (`self.Minutes`) 0 59)))
  (set `self.Minutes` _output_get_2)
  (bind _output_get_3 (set `self.Hours_0` (`KismetMathLibrary.Clamp` (`self.Hours`) 0 24)))
  (set `self.Hours` _output_get_3)
  (bind _returnvalue_2 (`KismetSystemLibrary.K2_SetTimerDelegate` (delegate `BranchDeath`) 1.0 true))
  (set `self.TH_TimerMission` _returnvalue_2))

(event `BranchDeath`
  (bind _baseplayerguard (`self.BasePlayerGuard`))
  (if (`self.GoMission`)
    (`/Engine/EditorBlueprintResources/StandardMacros.IsValid` _baseplayerguard
      (:`Is Valid`
        (if (`/Game/Postal2/Blueprint/Core/Character/BP_BaseNpcCharacter.bIsDeath` _baseplayerguard)
          (`/Engine/EditorBlueprintResources/StandardMacros.DoOnce` false
            (:`Completed`
              (set `self.MissionComplete` true)
              (`KismetSystemLibrary.Delay` 3.0)
              (`GameplayStatics.OpenLevel` "TownShops")
              (`KismetSystemLibrary.K2_ClearAndInvalidateTimerHandle` (`self.TH_TimerMission`))))
          (else
            (set `self.MissionComplete` false)))))))

(event `FinishOrFailed`
  (bind _returnvalue (`GameplayStatics.GetPlayerController` 0))
  (bind _wgtimer (`self.WGTimer`))
  (bind _text_close (`/Game/Postal2/Blueprint/Core/TimerMission/WG_Timer.Text_Close` _wgtimer))
  (bind _text_mission (`/Game/Postal2/Blueprint/Core/TimerMission/WG_Timer.Text_Mission` _wgtimer))
  (if (`self.MissionComplete`)
    (`Widget.SetVisibility` (`/Game/Postal2/Blueprint/Core/TimerMission/WG_Timer.Overlay_CompleteAndFailed` _wgtimer) "Visible")
    (`TextBlock.SetText` _text_mission "CompleteMission")
    (`TextBlock.SetText` _text_close "CloseQuest")
    (set `PlayerController.bShowMouseCursor` true _returnvalue)
    (`WidgetBlueprintLibrary.SetInputMode_UIOnlyEx` _returnvalue null)
    (else
      (`Widget.SetVisibility` (`/Game/Postal2/Blueprint/Core/TimerMission/WG_Timer.Overlay_CompleteAndFailed` (`self.WGTimer`)) "Visible")
      (`TextBlock.SetText` _text_mission "FailedMission")
      (`TextBlock.SetText` _text_close "Try again")
      (set `PlayerController.bShowMouseCursor` true _returnvalue)
      (`WidgetBlueprintLibrary.SetInputMode_UIOnlyEx` _returnvalue null)
      (set `self.Seconds` (`self.Seconds_0`))
      (set `self.Minutes` (`self.Minutes_0`))
      (set `self.Hours` (`self.Hours_0`))))
  (`Widget.SetVisibility` (`/Game/Postal2/Blueprint/Core/TimerMission/WG_Timer.Overlay_TimeMission` (`self.WGTimer`)) "Hidden")
  (`self.SetActorTickEnabled` false))

(event `self.ReceiveTick`
  (params (DeltaSeconds :type "Float (single-precision)"))
  (bind _seconds (`self.Seconds`))
  (if (`self.GoMission`)
    (if (== _seconds 0)
      (if (== (`self.Minutes`) 0)
        (if (== (`self.Hours`) 0)
          (`KismetSystemLibrary.Delay` 0.2)
          (`self.FinishOrFailed`)
          (else
            (set `self.Seconds` 59)
            (set `self.Minutes` 59)
            (bind _result (`/Engine/EditorBlueprintResources/StandardMacros.DecrementInt` (`self.Hours`))
              (:`  `
                (set `self.Hours` _result)))))
        (else
          (set `self.Seconds` 59)
          (bind _result_2 (`/Engine/EditorBlueprintResources/StandardMacros.DecrementInt` (`self.Minutes`))
            (:`  `
              (set `self.Minutes` _result_2)))))
      (else
        (bind _result_3 (`/Engine/EditorBlueprintResources/StandardMacros.DecrementInt` _seconds)
          (:`  `
            (set `self.Seconds` _result_3)))))))

(event `/Game/Postal2/Blueprint/Core/TimerMission/BPI_InteractQuest.Interaction`
  (params (`IsInteracted?` :type Boolean))
  (if `IsInteracted?`
    (`/Engine/EditorBlueprintResources/StandardMacros.DoOnce` false :!label _label
      (:`Completed`
        (bind _returnvalue (`|CreateWidget` "/Game/Postal2/Blueprint/Core/TimerMission/WG_Timer.WG_Timer_C"))
        (bind _output_get (set `self.WGTimer` _returnvalue))
        (`UserWidget.AddToViewport` _output_get 0)
        (set `self.GoMission` true)
        (`self.SetActorTickEnabled` true)
        (`KismetSystemLibrary.Delay` 5.0)
        (goto _label :!via `Reset`)))))

(fn `UserConstructionScript`)