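; BP_EnemySpawner is a placeable spawner that creates random enemy classes from Types on a looping timer.
; Each spawn lands at a random XY inside the collision box at its center height, facing the Arrow, and is skipped if collision can't be resolved.
; Spawning requires both the living-enemy count and the Types count to be below Limit.
; Spawned enemies are tracked through death-dispatcher bindings, freeing slots when they die.
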(event `self.ReceiveBeginPlay`
  (`KismetSystemLibrary.K2_SetTimerDelegate` (delegate `OnSpawnTimerTick`) (`self.Time`) true))

(event `OnSpawnTimerTick`
  (bind (_success _newenemy) (`self.SpawnNewEnemy`))
  (if _success
    (`KismetArrayLibrary.Array_Add` (`self.SpawnedEnemies`) _newenemy)
    (add `/Game/Postal2/Blueprint/Core/Character/BP_BaseCharacter.OnDeathDispather` _newenemy (delegate `OnSpawnEnemyDied`))))

(event `OnSpawnEnemyDied`
  (params (Source :type "/Game/Postal2/Blueprint/Core/Character/BP_BaseCharacter Object Reference"))
  (bind _asbp_base_npc_character (cast `/Game/Postal2/Blueprint/Core/Character/BP_BaseNpcCharacter` Source))
  (`KismetArrayLibrary.Array_RemoveItem` (`self.SpawnedEnemies`) _asbp_base_npc_character)
  (remove `/Game/Postal2/Blueprint/Core/Character/BP_BaseCharacter.OnDeathDispather` _asbp_base_npc_character (delegate `OnSpawnEnemyDied`)))

(fn `SpawnNewEnemy`
  (returns (Success :type Boolean) (NewEnemy :type "/Game/Postal2/Blueprint/Core/Character/BP_BaseNpcCharacter Object Reference"))
  (bind _returnvalue (`SceneComponent.K2_GetComponentLocation` (`self.CollisionBox`)))
  (if (and (< (`KismetArrayLibrary.Array_Length` (`self.Types`)) (`self.Limit`)) (< (`KismetArrayLibrary.Array_Length` (`self.SpawnedEnemies`)) (`self.Limit`)))
    (bind _returnvalue_2 (`|SpawnActorFromClass` (`KismetArrayLibrary.Array_Random` (`self.Types`)) (`KismetMathLibrary.MakeTransform` (`KismetMathLibrary.MakeVector` (.x (`KismetMathLibrary.RandomPointInBoundingBox` _returnvalue (`BoxComponent.GetScaledBoxExtent` (`self.CollisionBox`)))) (.y (`KismetMathLibrary.RandomPointInBoundingBox` _returnvalue (`BoxComponent.GetScaledBoxExtent` (`self.CollisionBox`)))) (.z _returnvalue)) (`SceneComponent.K2_GetComponentRotation` (`self.Arrow`))) "AdjustIfPossibleButDontSpawnIfColliding" "MultiplyWithRoot" null null))
    (`/Engine/EditorBlueprintResources/StandardMacros.IsValid` _returnvalue_2
      (:`Is Valid`
        (return true _returnvalue_2))
      (:`Is Not Valid`
        (return false null)))
    (else
      (return false null))))

(fn `UserConstructionScript`)